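; Player controller that returns the player to the game mode's saved checkpoint when R is pressed.
; It reads the Checkpoint from BP_ThirdPersonGameMode and, if valid, moves the player character to that location and rotation.
; A branch to spawn and possess a new BP_ThirdPersonCharacter there never runs, as its condition is fixed to true and the character validity check is unconnected.
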(event `Key|R`
  (params (Key :type "Key Structure"))
  (:`Pressed`
    (bind _asbp_third_person_game_mode (cast `/Game/ThirdPerson/Blueprints/BP_ThirdPersonGameMode` (`GameplayStatics.GetGameMode`)))
    (bind _checkpoint (`/Game/ThirdPerson/Blueprints/BP_ThirdPersonGameMode.Checkpoint` _asbp_third_person_game_mode)
      (:`then`
        (if true
          (bind _returnvalue (`self.K2_GetActorLocation` _checkpoint))
          (bind _returnvalue_2 (`self.K2_GetActorRotation` _checkpoint))
          (`self.K2_SetActorLocationAndRotation` (`GameplayStatics.GetPlayerCharacter` 0) _returnvalue _returnvalue_2 false false)
          (else
            (bind _returnvalue_3 (`|SpawnActorFromClass` "/Game/ThirdPerson/Blueprints/BP_ThirdPersonCharacter.BP_ThirdPersonCharacter_C" (`KismetMathLibrary.MakeTransform` _returnvalue _returnvalue_2) "Undefined" "MultiplyWithRoot" null null))
            (`self.Possess` _returnvalue_3))))
      (:`else`))))

(fn `UserConstructionScript`)