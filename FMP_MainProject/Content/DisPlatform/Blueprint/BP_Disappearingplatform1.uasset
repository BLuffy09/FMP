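; BP_Disappearingplatform1 is a platform that fades and drops its collision when the third-person character enters its trigger box, then restores itself.
; BeginPlay creates a dynamic material instance on the floor mesh for the timelines to drive.
; One timeline animates Opacity before collision is disabled, then a second animates it before collision returns.
; An IsDisapearing flag blocks retriggering until the cycle finishes.
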(event `self.ReceiveBeginPlay`
  (bind _returnvalue (`PrimitiveComponent.CreateDynamicMaterialInstance` (`self.Floor`) 0 "/Game/DisPlatform/Material/M_Disapearingfloor.M_Disapearingfloor" "None"))
  (bind _output_get (set `self.Material Instance` _returnvalue))
  (`MaterialInstanceDynamic.SetScalarParameterValue` _output_get "Disapearingfloor" 0.0))

(event `self.Box.OnComponentBeginOverlap`
  (params (OverlappedComponent :type "PrimitiveComponent Object Reference") (OtherActor :type "Actor Object Reference") (OtherComp :type "PrimitiveComponent Object Reference") (OtherBodyIndex :type Integer) (bFromSweep :type Boolean) (SweepResult :type "HitResult Structure (by ref)"))
  (cast `/Game/ThirdPerson/Blueprints/BP_ThirdPersonCharacter` OtherActor)
  (if (not (`self.IsDisapearing`))
    (set `self.IsDisapearing` true)
    (bind (_direction _disapearingfloattrack) (`Timeline|Disapearingfloortime` :!via `PlayFromStart`)
      (:`Update`
        (`MaterialInstanceDynamic.SetScalarParameterValue` (`self.Material Instance`) "Opacity" _disapearingfloattrack))
      (:`Finished`
        (`PrimitiveComponent.SetCollisionEnabled` (`self.Floor`) "NoCollision")
        (bind (_direction_2 _disapearingfloattrack_2) (`Timeline|Timeline` :!via `PlayFromStart`)
          (:`Update`
            (`MaterialInstanceDynamic.SetScalarParameterValue` (`self.Material Instance`) "Opacity" _disapearingfloattrack_2))
          (:`Finished`
            (`PrimitiveComponent.SetCollisionEnabled` (`self.Floor`) "QueryAndPhysics")
            (set `self.IsDisapearing` false)))))))

(fn `UserConstructionScript`)