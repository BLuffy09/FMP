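; Interactive keypad actor that the player uses to enter a numeric code with mouse clicks.
; Interacting switches the view to the keypad, locks movement and look, and enables click events; Q restores control through the exit macro.
; Digit button clicks append to the input via CODE, which plays a sound and updates the widget text.
; A correct code turns the spheres green, flags the character and releases control; input clears after five digits.
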(event `self.ReceiveBeginPlay`
  (bind _aswbp_keypad (cast `/Game/WBP_Keypad` (`WidgetComponent.GetWidget` (`self.Widget`))))
  (set `self.As WBP Keypad` _aswbp_keypad))

(event `self.E-interact`
  (bind _returnvalue (`GameplayStatics.GetPlayerController` 0))
  (bind _returnvalue_2 (`GameplayStatics.GetPlayerController` 0))
  (`PlayerController.SetViewTargetWithBlend` _returnvalue_2 self 0.0 "VTBlend_Linear" 0.0 false)
  (`Controller.SetIgnoreLookInput` _returnvalue_2 true)
  (set `PlayerController.bEnableClickEvents` true _returnvalue_2)
  (set `PlayerController.bShowMouseCursor` true _returnvalue_2)
  (`CharacterMovementComponent.DisableMovement` (`Character.CharacterMovement` (`GameplayStatics.GetPlayerCharacter` 0)))
  (`self.EnableInput` _returnvalue)
  (`WidgetBlueprintLibrary.SetInputMode_GameAndUIEx` _returnvalue null))

(event `Key|Q`
  (params (Key :type "Key Structure"))
  (bind _returnvalue (`GameplayStatics.GetPlayerController` 0))
  (:`Pressed`
    (`PlayerController.SetViewTargetWithBlend` _returnvalue (`GameplayStatics.GetPlayerCharacter` 0) 0.0 "VTBlend_Linear" 0.0 false)
    (`Controller.ResetIgnoreLookInput` _returnvalue)
    (set `PlayerController.bEnableClickEvents` false _returnvalue)
    (set `PlayerController.bShowMouseCursor` false _returnvalue)
    (`CharacterMovementComponent.SetMovementMode` (`Character.CharacterMovement` (`GameplayStatics.GetPlayerCharacter` 0)) "MOVE_Walking" 0)
    (`WidgetBlueprintLibrary.SetInputMode_GameOnly` _returnvalue)
    (`self.DisableInput` _returnvalue)))

(event `self.button1.OnClicked`
  (params (TouchedComponent :type "PrimitiveComponent Object Reference") (ButtonPressed :type "Key Structure"))
  (`self.CODE` "1"))

(event `self.button6.OnClicked`
  (params (TouchedComponent :type "PrimitiveComponent Object Reference") (ButtonPressed :type "Key Structure"))
  (`self.CODE` "6"))

(event `self.button2.OnClicked`
  (params (TouchedComponent :type "PrimitiveComponent Object Reference") (ButtonPressed :type "Key Structure"))
  (`self.CODE` "2"))

(event `self.button7.OnClicked`
  (params (TouchedComponent :type "PrimitiveComponent Object Reference") (ButtonPressed :type "Key Structure"))
  (`self.CODE` "7"))

(event `self.button3.OnClicked`
  (params (TouchedComponent :type "PrimitiveComponent Object Reference") (ButtonPressed :type "Key Structure"))
  (`self.CODE` "3"))

(event `self.button8.OnClicked`
  (params (TouchedComponent :type "PrimitiveComponent Object Reference") (ButtonPressed :type "Key Structure"))
  (`self.CODE` "8"))

(event `self.button4.OnClicked`
  (params (TouchedComponent :type "PrimitiveComponent Object Reference") (ButtonPressed :type "Key Structure"))
  (`self.CODE` "4"))

(event `self.button9.OnClicked`
  (params (TouchedComponent :type "PrimitiveComponent Object Reference") (ButtonPressed :type "Key Structure"))
  (`self.CODE` "9"))

(event `self.button5.OnClicked`
  (params (TouchedComponent :type "PrimitiveComponent Object Reference") (ButtonPressed :type "Key Structure"))
  (`self.CODE` "5"))

(fn `CODE`
  (params (B :type String))
  (bind _returnvalue (`GameplayStatics.GetPlayerController` 0))
  (bind _returnvalue_2 (`GameplayStatics.GetPlayerCharacter` 0))
  (`GameplayStatics.PlaySound2D` "/Game/VehicleTemplate/keypad_materials/key_code_sfx.key_code_sfx" 1.0 1.0 0.0 null null)
  (bind _output_get (set `self.input` (`KismetStringLibrary.Concat_StrStr` (`self.input`) B)))
  (set `self.length_of_code` (+ (`self.length_of_code`) 1))
  (`TextBlock.SetText` (`/Game/WBP_Keypad.codetext` (`self.As WBP Keypad`)) (`KismetTextLibrary.Conv_StringToText` _output_get))
  (if (`KismetStringLibrary.EqualEqual_StrStr` (`self.input`) (`self.Correct code`))
    (message `/Game/BPI_UNLOCK_DOOR.set code correct` (`GameplayStatics.GetPlayerCharacter` 0) true)
    (`PrimitiveComponent.SetMaterial` (`self.spheres`) 0 "/Game/MK_GRRREEEEEEEEN.MK_GRRREEEEEEEEN")
    (`self.DisableInput` _returnvalue)
    (`PlayerController.SetViewTargetWithBlend` _returnvalue _returnvalue_2 0.3 "VTBlend_Linear" 0.0 false)
    (`Controller.ResetIgnoreLookInput` _returnvalue)
    (set `PlayerController.bEnableClickEvents` false _returnvalue)
    (set `PlayerController.bShowMouseCursor` false _returnvalue)
    (`CharacterMovementComponent.SetMovementMode` (`Character.CharacterMovement` _returnvalue_2) "MOVE_Walking" 0)
    (`WidgetBlueprintLibrary.SetInputMode_GameOnly` _returnvalue))
  (if (>= (`self.length_of_code`) 5)
    (bind _output_get_2 (set `self.input` ""))
    (`TextBlock.SetText` (`/Game/WBP_Keypad.codetext` (`self.As WBP Keypad`)) (`KismetTextLibrary.Conv_StringToText` _output_get_2))
    (set `self.length_of_code` 0)))

(fn `UserConstructionScript`)